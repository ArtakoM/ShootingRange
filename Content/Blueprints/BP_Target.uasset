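; BP_Target is a target actor that, when MovingTarget is set, moves every tick and bounces back on contact with walls.
; Each tick it teleports by SumVector from the static mesh's world location, without sweep or delta-time scaling.
; A multi-object line trace across the diagonal of the actor's bounds detects walls, and any hit negates the Y component of SumVector to reverse lateral movement.
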(event EventTick
  (params (DeltaSeconds :type Float%20%28single-precision%29))
  (if (Variables|Default|GetMovingTarget?)
    (CallFunction|MoveTraget)
    (bind _istouching (CallFunction|DetectWallTouch))
    (CallFunction|SetMoveDirection _istouching)))

(fn ConstructionScript)

(fn MoveTraget
  (Transformation|SetActorLocation (+ (Transformation|GetWorldLocation (Variables|Default|GetStaticMesh)) (Variables|Default|GetSumVector)) false false))

(fn DetectWallTouch
  (bind (_origin _boxextent) (Collision|GetActorBounds false false))
  (bind _returnvalue (Class|KismetSystemLibrary|LineTraceMultiforObjects (- _origin _boxextent) (+ _origin _boxextent) (Variables|Default|GetObject%20Types) false 0 "None" true))
  (return _returnvalue))

(fn SetMoveDirection
  (params (Condition :type Boolean))
  (if Condition
    (Variables|Default|SetSumVector (* (Variables|Default|GetSumVector) "1.000000,-1.000000,1.000000"))))